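; Player controller that builds the HUD and menus for what appears to be a wave-based tower game.
; On BeginPlay it creates the escape menu, currency display, intermission timer, game over, tower select and purchase widgets for player 0 and adds them to the viewport.
; It stores the three menus and initializes their visibility, starting the escape menu with false.
; Escape or O toggles the escape menu based on its current visibility.
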(event EventBeginPlay
  (bind _returnvalue (Class|GameplayStatics|GetPlayerControllerfromID))
  (bind _returnvalue_2 (UserInterface|CreateWidget "/Game/UI/WBP_EscapeMenu.WBP_EscapeMenu_C" (Class|GameplayStatics|GetPlayerControllerfromID)))
  (bind _output_get (Variables|Default|SetEscapeMenu _returnvalue_2))
  (Default|UpdateVisibility _output_get false)
  (UserInterface|Viewport|AddtoViewport _output_get 0)
  (bind _returnvalue_3 (UserInterface|CreateWidget "/Game/UI/WBP_CurrencyDisplay.WBP_CurrencyDisplay_C" (Class|GameplayStatics|GetPlayerControllerfromID)))
  (UserInterface|Viewport|AddtoViewport _returnvalue_3 0)
  (bind _returnvalue_4 (UserInterface|CreateWidget "/Game/UI/WBP_WaveIntermissionTimer.WBP_WaveIntermissionTimer_C" _returnvalue))
  (UserInterface|Viewport|AddtoViewport _returnvalue_4 0)
  (bind _returnvalue_5 (UserInterface|CreateWidget "/Game/UI/WBP_GameOver.WBP_GameOver_C" _returnvalue))
  (UserInterface|Viewport|AddtoViewport _returnvalue_5 0)
  (bind _returnvalue_6 (UserInterface|CreateWidget "/Game/UI/TowerSelectMenu/WBP_TowerSelectMenu.WBP_TowerSelectMenu_C" _returnvalue))
  (bind _output_get_2 (Variables|Default|SetTowerSelectMenu _returnvalue_6))
  (UserInterface|Viewport|AddtoViewport _output_get_2 0)
  (Default|UpdateVisibility _output_get_2)
  (bind _returnvalue_7 (UserInterface|CreateWidget "/Game/UI/TowerSelectMenu/WBP_PurchaseMenu.WBP_PurchaseMenu_C" _returnvalue))
  (bind _output_get_3 (Variables|Default|SetPurchaseMenu _returnvalue_7))
  (UserInterface|Viewport|AddtoViewport _output_get_3 0)
  (Default|UpdateVisibility _output_get_3))

(event EventTick
  (params (DeltaSeconds :type Float%20%28single-precision%29)))

(event Input|KeyboardEvents|O
  (params (Key :type Key%20Structure :default "None"))
  (bind _escapemenu (Variables|Default|GetEscapeMenu))
  (:Pressed
    (switch Utilities|FlowControl|Switch|SwitchonESlateVisibility (Widget|GetVisibility (Variables|Default|GetEscapeMenu))
      (:Visible
        (Default|UpdateVisibility _escapemenu false))
      (:Collapsed
        (Default|UpdateVisibility _escapemenu true :!label _label))
      (:Hidden
        (goto _label)))))

(event Input|KeyboardEvents|Escape
  (params (Key :type Key%20Structure :default "None"))
  (bind _escapemenu (Variables|Default|GetEscapeMenu))
  (:Pressed
    (switch Utilities|FlowControl|Switch|SwitchonESlateVisibility (Widget|GetVisibility (Variables|Default|GetEscapeMenu))
      (:Visible
        (Default|UpdateVisibility _escapemenu false))
      (:Collapsed
        (Default|UpdateVisibility _escapemenu true :!label _label))
      (:Hidden
        (goto _label)))))

(fn ConstructionScript)