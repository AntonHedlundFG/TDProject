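; BP_SingleHitScanProjectile is a tower projectile Blueprint that displays a laser beam with an impact effect.
; On BeginPlay it runs the parent logic, then sets both effects' colors and the beam's width through named parameters.
; SpawnLaserBeam moves the beam end and impact to the given point, then reveals both after a very short delay.
; HideLaserBeam hides both, so the same components are toggled rather than spawned.
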(event EventBeginPlay
  (bind _returnvalue (Utilities|String|MakeLiteralString "Color"))
  (bind _returnvalue_2 (Utilities|String|StringToName _returnvalue))
  (|CallParentFunction)
  (Effects|Components|ParticleSystem|SetColorParameter (Variables|Default|GetImpact) _returnvalue_2 "(R=0.008418,G=0.000000,B=1.000000,A=1.000000)")
  (Effects|Components|ParticleSystem|SetColorParameter (Variables|Default|GetBeam) _returnvalue_2 "(R=0.053686,G=0.000000,B=1.000000,A=1.000000)")
  (Effects|Components|ParticleSystem|SetFloatParameter (Variables|Default|GetBeam) "Width" 15.0))

(event EventSpawnLaserBeam
  (params (End :type Vector :default "0, 0, 0"))
  (Effects|Components|ParticleSystem|SetVectorParameter (Variables|Default|GetBeam) "BeamEnd" End)
  (Transformation|SetWorldLocation (Variables|Default|GetImpact) End false true)
  (Utilities|FlowControl|Delay 0.01)
  (Rendering|SetVisibility (Variables|Default|GetBeam) true true)
  (Rendering|SetVisibility (Variables|Default|GetImpact) true true))

(event EventHideLaserBeam
  (Rendering|SetVisibility (Variables|Default|GetBeam) false true)
  (Rendering|SetVisibility (Variables|Default|GetImpact) false true))

(fn ConstructionScript
  (|CallParentFunction))