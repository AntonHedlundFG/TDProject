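; BP_TowerBase is a base tower Blueprint that opens a purchase menu when a player interacts with it.
; LocalInteractBP acts only if the tower has Purchasables and the user casts to BP_PlayerController.
; It then has that controller's PurchaseMenu generate buttons from the tower, records the user and updates the menu's visibility.
; BeginPlay and the construction script only call their parent versions.
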(event EventBeginPlay
  (|CallParentFunction))

(event EventLocalInteractBP
  (params (User :type Player%20Controller%20Object%20Reference) (Param :type Byte :default 0))
  (if (> (Utilities|Array|Length (Variables|Default|GetPurchasables)) 0)
    (bind _asbp_player_controller (Utilities|Casting|CastToBP_PlayerController User))
    (Default|GenerateButtons (Variables|/Game/Levels/BP_PlayerController.BP_PlayerController_C|GetPurchaseMenu _asbp_player_controller) self)
    (Variables|/Game/UI/TowerSelectMenu/WBP_PurchaseMenu.WBP_PurchaseMenu_C|SetUser (Variables|/Game/Levels/BP_PlayerController.BP_PlayerController_C|GetPurchaseMenu _asbp_player_controller) User)
    (Default|UpdateVisibility (Variables|/Game/Levels/BP_PlayerController.BP_PlayerController_C|GetPurchaseMenu _asbp_player_controller))))

(fn ConstructionScript
  (|CallParentFunction))