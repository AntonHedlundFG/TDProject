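; Laser tower Blueprint that supplies beam and impact visuals for shots and a purchase menu on interaction.
; The beam is colored, sized and hidden on BeginPlay, then shown to a given end point or hidden through shot visual events.
; Impacts spawn a pooled, short-lived Niagara effect at the hit location.
; Local interaction fills the player controller's purchase menu with this tower's buttons and updates its visibility.
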(event EventBeginPlay
  (bind _beam (Variables|Default|GetBeam))
  (|CallParentFunction)
  (Effects|Components|ParticleSystem|SetColorParameter _beam (Utilities|String|StringToName (Utilities|String|MakeLiteralString "Color")) "(R=0.053686,G=0.000000,B=1.000000,A=1.000000)")
  (Effects|Components|ParticleSystem|SetFloatParameter _beam "Width" 15.0)
  (Rendering|SetVisibility (Variables|Default|GetBeam) false true))

(event Collision|EventActorBeginOverlap
  (params (OtherActor :type Actor%20Object%20Reference)))

(event EventTick
  (params (DeltaSeconds :type Float%20%28single-precision%29)))

(event EventShowImpactVisual
  (params (Location :type Vector :default "0, 0, 0"))
  (bind _returnvalue (Niagara|SpawnSystematLocation "/Game/Particles/NiagaraSystems/NS_LaserImpact.NS_LaserImpact" Location "0, 0, 0" "1.000000,1.000000,1.000000" false true "AutoRelease"))
  (Effects|Components|ParticleSystem|SetFloatParameter _returnvalue "LifeTime" 0.25))

(event EventLocalInteractBP
  (params (User :type Player%20Controller%20Object%20Reference) (Param :type Byte :default 0))
  (bind _asbp_player_controller (Utilities|Casting|CastToBP_PlayerController User))
  (Default|GenerateButtons (Variables|/Game/Levels/BP_PlayerController.BP_PlayerController_C|GetPurchaseMenu _asbp_player_controller) self)
  (Variables|/Game/UI/TowerSelectMenu/WBP_PurchaseMenu.WBP_PurchaseMenu_C|SetUser (Variables|/Game/Levels/BP_PlayerController.BP_PlayerController_C|GetPurchaseMenu _asbp_player_controller) User)
  (Default|UpdateVisibility (Variables|/Game/Levels/BP_PlayerController.BP_PlayerController_C|GetPurchaseMenu _asbp_player_controller)))

(event EventShowShotVisual
  (params (Start :type Vector :default "0, 0, 0") (End :type Vector :default "0, 0, 0"))
  (bind _beam (Variables|Default|GetBeam))
  (Effects|Components|ParticleSystem|SetVectorParameter _beam "BeamEnd" End)
  (Rendering|SetVisibility _beam true true))

(event EventHideShotVisual
  (Rendering|SetVisibility (Variables|Default|GetBeam) false true))

(fn ConstructionScript
  (|CallParentFunction))