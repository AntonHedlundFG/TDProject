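; Sniper tower Blueprint that draws its shots as fading laser trails and opens the purchase menu when a player interacts with it.
; ShowShotVisual spawns a manually pooled Niagara beam between start and end points, releasing any previous one first.
; A Delay loop steps the projectile color's alpha down over FadeTime, then returns the beam to the pool.
; LocalInteractBP fills the player controller's purchase menu for this tower and updates its visibility.
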(event EventBeginPlay
  (|CallParentFunction))

(event Collision|EventActorBeginOverlap
  (params (OtherActor :type Actor%20Object%20Reference)))

(event EventTick
  (params (DeltaSeconds :type Float%20%28single-precision%29)))

(event EventLocalInteractBP
  (params (User :type Player%20Controller%20Object%20Reference) (Param :type Byte :default 0))
  (bind _asbp_player_controller (Utilities|Casting|CastToBP_PlayerController User))
  (Default|GenerateButtons (Variables|/Game/Levels/BP_PlayerController.BP_PlayerController_C|GetPurchaseMenu _asbp_player_controller) self)
  (Variables|/Game/UI/TowerSelectMenu/WBP_PurchaseMenu.WBP_PurchaseMenu_C|SetUser (Variables|/Game/Levels/BP_PlayerController.BP_PlayerController_C|GetPurchaseMenu _asbp_player_controller) User)
  (Default|UpdateVisibility (Variables|/Game/Levels/BP_PlayerController.BP_PlayerController_C|GetPurchaseMenu _asbp_player_controller)))

(event EventShowShotVisual
  (params (Start :type Vector :default "0, 0, 0") (End :type Vector :default "0, 0, 0"))
  (bind _returnvalue (Math|Float|MakeLiteralFloat 0.1))
  (bind _spawnedtrail (CallFunction|SpawnBulletTrail Start))
  (bind _output_get (Variables|Default|SetBeam _spawnedtrail))
  (Effects|Components|ParticleSystem|SetFloatParameter _output_get "Width" (Variables|Default|GetBeamWidth))
  (Effects|Components|ParticleSystem|SetVectorParameter _output_get "BeamEnd" End)
  (Rendering|SetVisibility _output_get true true)
  (Variables|Default|SetCurrentColor (.color (Variables|/Script/Angelscript.TowerData|GetProjectileData (Variables|Default|GetTowerData))))
  (bind _bisdone (CallFunction|FadeOutTrail _returnvalue :!label _label))
  (Utilities|FlowControl|Delay _returnvalue)
  (if _bisdone
    (goto _label)
    (else
      (Effects|Components|ParticleSystem|ReleasetoPool (Variables|Default|GetBeam)))))

(event EventHideShotVisual
  (Rendering|SetVisibility (Variables|Default|GetBeam) false true))

(fn ConstructionScript
  (|CallParentFunction))

(fn SpawnBulletTrail
  (params (Location :type Vector))
  (bind _beam (Variables|Default|GetBeam))
  (if (Utilities|IsValid _beam)
    (Effects|Components|ParticleSystem|ReleasetoPool _beam))
  (bind _returnvalue (Niagara|SpawnSystematLocation "/Game/Particles/NiagaraSystems/NS_Laser.NS_Laser" Location "0, 0, 0" "1.000000,1.000000,1.000000" true true "ManualRelease"))
  (return _returnvalue))

(fn FadeOutTrail
  (params (Percent :type Float%20%28double-precision%29))
  (bind _returnvalue (Math|Float|MakeLiteralFloat Percent))
  (bind _fadetime (Variables|Default|GetFadeTime))
  (bind _returnvalue_2 (/ 1.0 _fadetime))
  (bind _returnvalue_3 (* _returnvalue _returnvalue_2))
  (Effects|Components|ParticleSystem|SetColorParameter (Variables|Default|GetBeam) "Color" (Variables|Default|GetCurrentColor))
  (Variables|Default|SetCurrentColor (Utilities|Struct|MakeLinearColor (.r (Variables|Default|GetCurrentColor)) (.g (Variables|Default|GetCurrentColor)) (.b (Variables|Default|GetCurrentColor)) (- (.a (Variables|Default|GetCurrentColor)) _returnvalue_3)))
  (return (> (- (.a (Variables|Default|GetCurrentColor)) _returnvalue_3) (* _returnvalue_3 -2.0))))