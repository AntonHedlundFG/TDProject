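; BP_EnemyBasic is a basic enemy with a health bar and a physics-constrained mesh.
; On BeginPlay it initializes the health bar widget from the HealthSystemComponent and binds to its health-change event to keep the bar updated.
; A physics constraint links the mesh to a root component, while Tick applies a constant upward force to the mesh.
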(event Custom|CustomEvent
  (params (CurrentHealth :type Integer) (MaxHealth :type Integer))
  ;[1 1 1] HealthBar Setup
  (Class|HealthBarWidget|UpdateHealthBar (stale EventBeginPlay _ashealth_bar_widget) CurrentHealth MaxHealth))

(event EventBeginPlay
  (bind _healthsystemcomponent (Variables|Default|GetHealthSystemComponent))
  (|CallParentFunction)
  ;[1 1 1] HealthBar Setup
  (bind _ashealth_bar_widget (Utilities|Casting|CastToHealthBarWidget (UserInterface|GetWidget (Variables|Default|GetHealthBarWidgetComponent)))
    (:then
      (EventDispatchers|AssignOnHealthChanged (Variables|Default|GetHealthSystemComponent) (delegate Custom|CustomEvent))
      (Class|HealthBarWidget|UpdateHealthBar _ashealth_bar_widget (Variables|/Script/Angelscript.HealthSystemComponent|GetCurrentHealth _healthsystemcomponent) (Variables|/Script/Angelscript.HealthSystemComponent|GetMaxHealth _healthsystemcomponent)))
    (:CastFailed
      _))
  (Class|PhysicsConstraintComponent|SetConstrainedComponents (Variables|Default|GetPhysicsConstraint) (Variables|Default|GetPhysicsConstraintRoot) "None" (Variables|Character|GetMesh) "None"))

(event EventTick
  (params (DeltaSeconds :type Float%20%28single-precision%29))
  (bind _mesh (Variables|Character|GetMesh))
  (|CallParentFunction DeltaSeconds)
  (Utilities|IsValid _mesh
    (:Is%20Valid
      (Physics|AddForce _mesh "0.000000,0.000000,500.000000" "None" false))))

(fn ConstructionScript
  (|CallParentFunction))